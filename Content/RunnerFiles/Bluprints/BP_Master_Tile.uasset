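; BP_Master_Tile is a track tile for an endless runner that extends the course as the player advances.
; On BeginPlay it has a one-in-four chance of spawning a fence obstacle at Lane0, the only lane handled here.
; When the character overlaps its Box, it asks the game mode to spawn another tile and add a point, increases the player's velocity, then destroys itself after a short delay.
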(event OnComponentBeginOverlap(Box)
  (params (OverlappedComponent :type Primitive%20Component%20Object%20Reference) (OtherActor :type Actor%20Object%20Reference) (OtherComp :type Primitive%20Component%20Object%20Reference) (OtherBodyIndex :type Integer) (bFromSweep :type Boolean) (SweepResult :type Hit%20Result%20Structure%20%28by%20ref%29))
  ;[1 1 1] Cria uma nova pista de corrida
  (Utilities|Casting|CastToThirdPersonCharacter OtherActor)
  (bind _asthird_person_game_mode (Utilities|Casting|CastToThirdPersonGameMode (Game|GetGameMode)))
  (Default|SpawnTile _asthird_person_game_mode)
  (Default|AddPoints _asthird_person_game_mode 1)
  (bind _asthird_person_character (Utilities|Casting|CastToThirdPersonCharacter (Game|GetPlayerCharacter 0)))
  (Default|IncVelocity _asthird_person_character)
  (Utilities|FlowControl|Delay 3.0)
  (Actor|DestroyActor))

(event EventBeginPlay
  (CallFunction|SpawnObstacle))

(event Collision|EventActorBeginOverlap
  (params (OtherActor :type Actor%20Object%20Reference)))

(event EventTick
  (params (DeltaSeconds :type Float%20%28single-precision%29)))

(fn ConstructionScript)

(fn SpawnObstacle
  ;[1 1 1] Line 0 - Pista 1
  (switch int (Math|Random|RandomIntegerinRange 0 3)
    (:0
      (Game|SpawnActorfromClass "/Game/RunnerFiles/Bluprints/BP_ObstacleFence.BP_ObstacleFence_C" (Transformation|GetWorldTransform (Variables|Default|GetLane0)) "Undefined" 0 0))))