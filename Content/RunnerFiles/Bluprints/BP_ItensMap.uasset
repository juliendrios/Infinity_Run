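; BP_ItensMap is a map decoration actor for the runner game that randomly varies which scenery prop appears at its location.
; On BeginPlay, a random integer drives a switch that makes one of ten components visible: trees, flowers, plants or rocks.
; The random range includes zero, which has no case, so sometimes the actor reveals nothing.
; The graph only turns visibility on, with no spawning or per-tick logic.
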(event EventBeginPlay
  (switch int (Math|Random|RandomInteger 11)
    (:1
      ;[1 0.2526 0.1729] Itens_Randomico_No_Mapa
      (Rendering|SetVisibility (Variables|Default|Getarvore1) true false))
    (:2
      (Rendering|SetVisibility (Variables|Default|Getarvore2) true false))
    (:3
      (Rendering|SetVisibility (Variables|Default|Getarvore3) true false))
    (:4
      (Rendering|SetVisibility (Variables|Default|Getarvore4) true false))
    (:5
      (Rendering|SetVisibility (Variables|Default|Getflor1) true false))
    (:6
      (Rendering|SetVisibility (Variables|Default|Getflor2) true false))
    (:7
      (Rendering|SetVisibility (Variables|Default|Getplanta1) true false))
    (:8
      (Rendering|SetVisibility (Variables|Default|Getplanta2) true false))
    (:9
      (Rendering|SetVisibility (Variables|Default|Getpedra1) true false))
    (:10
      (Rendering|SetVisibility (Variables|Default|Getpedra2) true false))))

(event Collision|EventActorBeginOverlap
  (params (OtherActor :type Actor%20Object%20Reference)))

(event EventTick
  (params (DeltaSeconds :type Float%20%28single-precision%29)))

(fn ConstructionScript)